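; BP_Bird is a flying enemy character that dives at the player and knocks them back on contact.
; Attack extends the parent's, launching the bird toward player zero and setting a short timer, while StopLaunch halts movement and restores Flying mode.
; Capsule overlap with BP_BombieJackieCharacter runs HandleDeath first, then, if unhandled and Attacking, launches the character along the mesh's forward vector with upward lift.
; The construction script records the spawn position as RestingLocation.
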(event OnComponentBeginOverlap(CapsuleComponent)
  (params (OverlappedComponent :type Primitive%20Component%20Object%20Reference) (OtherActor :type Actor%20Object%20Reference) (OtherComp :type Primitive%20Component%20Object%20Reference) (OtherBodyIndex :type Integer) (bFromSweep :type Boolean) (SweepResult :type Hit%20Result%20Structure%20%28by%20ref%29))
  (bind _mesh (Variables|Character|GetMesh))
  (bind _returnvalue (Math|Vector|GetForwardVector _mesh))
  (bind _asbp_bombie_jackie_character (Utilities|Casting|CastToBP_BombieJackieCharacter OtherActor))
  (bind _enemydied (CallFunction|HandleDeath _asbp_bombie_jackie_character))
  (if (not _enemydied)
    (if (Variables|Default|GetAttacking)
      (Character|LaunchCharacter _asbp_bombie_jackie_character (* (Math|Vector|MakeVector (.x _returnvalue) (.y _returnvalue) 1.0) (Variables|Default|GetKnockbackStrength)) true true))))

(event Custom|StopLaunch
  (Components|Movement|StopMovementImmediately (Variables|Character|GetCharacterMovement))
  (Pawn|Components|CharacterMovement|SetMovementMode (Variables|Character|GetCharacterMovement) "MOVE_Flying" 0))

(event EventBeginPlay
  (|CallParentFunction))

(event Collision|EventActorBeginOverlap
  (params (OtherActor :type Actor%20Object%20Reference))
  (|CallParentFunction OtherActor) ; This node is disabled and will not be called.\nDrag off pins to build functionality.
)

(event EventTick
  (params (DeltaSeconds :type Float%20%28single-precision%29))
  (|CallParentFunction DeltaSeconds) ; This node is disabled and will not be called.\nDrag off pins to build functionality.
)

(fn ConstructionScript
  (|CallParentFunction)
  (Variables|Default|SetRestingLocation (Transformation|GetActorLocation)))

(fn Attack
  (|CallParentFunction)
  (Character|LaunchCharacter self (* (Math|Vector|Normalize (- (Transformation|GetActorLocation (Game|GetPlayerCharacter 0)) (Transformation|GetActorLocation))) (Variables|Default|GetLaunchStrength)) true true)
  (Utilities|Time|SetTimerbyEvent (EventDispatchers|CreateEvent :!event Custom|StopLaunch) 1.0))