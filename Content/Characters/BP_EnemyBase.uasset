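; Base enemy character with zombie-style groans, sight-based player detection, an attack cooldown and a special death condition.
; AI perception sight stimuli update whether it sees the player and send a seen event to its StateTree on success.
; Attack sets an attacking flag, starts a cooldown timer and plays attached audio, while idle sounds loop on randomized timers.
; Capsule hits from a player both dashing and in super state destroy it with Niagara and sound effects.
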(event OnTargetPerceptionUpdated(AIPerception)
  (params (Actor :type Actor%20Object%20Reference) (Stimulus :type AI%20Stimulus%20Structure))
  ;[0.15 0 0.02195 0.5] Handle the enemy detecting the player
  (bind _successfullysensed (CallFunction|HandleSightSense Actor Stimulus))
  (bind _output_get (Variables|Default|SetIsSeeingThePlayer _successfullysensed))
  (if _output_get
    (Gameplay|StateTree|SendStateTreeEvent (Variables|Default|GetStateTree) (Variables|Default|GetSeenEvent) :!class /Script/GameplayStateTreeModule.StateTreeComponent)))

(event OnComponentHit(CapsuleComponent)
  (params (HitComponent :type Primitive%20Component%20Object%20Reference) (OtherActor :type Actor%20Object%20Reference) (OtherComp :type Primitive%20Component%20Object%20Reference) (NormalImpulse :type Vector :default "0, 0, 0") (Hit :type Hit%20Result%20Structure%20%28by%20ref%29))
  ;[0.15 0.15 0.15 0.5] Murder Enemy
  (bind _asbp_bombie_jackie_character (Utilities|Casting|CastToBP_BombieJackieCharacter OtherActor))
  (CallFunction|HandleDeath _asbp_bombie_jackie_character))

(event Custom|RestartIdleSoundTimer
  (params (Time :type Float%20%28double-precision%29))
  ;[0 0.001015 0.15 0.5] Place random sound from the sound cue, and restarts the timer for a new badie sound
  (Utilities|Time|SetTimerbyEvent (delegate Custom|PlayIdleSound) Time))

(event Custom|OnAttackCooldownFinished
  ;[0.15 0 0.1094 0.5] Reset attack cooldown
  (Variables|Default|SetAttacking false))

(event Custom|PlayIdleSound
  ;[0 0.001015 0.15 0.5] Place random sound from the sound cue, and restarts the timer for a new badie sound
  (Audio|SpawnSoundAttached (Variables|Default|GetIdleSounds) (Variables|Character|GetMesh) "None" "0, 0, 0" "0, 0, 0" "KeepRelativeOffset" false 1.0 1.0 0.0 "/Game/Characters/Zombie/Audio/SA_ZombieGroan.SA_ZombieGroan" 0)
  (CallFunction|RestartIdleSoundTimer (Math|Random|RandomFloatinRange (Variables|Default|GetMinTimeBetweenIdleSoundPlay) (Variables|Default|GetMaxTimeBetweenIdleSoundPlay))))

(event EventBeginPlay
  ;[0.15 0.1054 0 0.5] Starts timer for when to play random noices from the badies
  (if (Utilities|IsValid (Variables|Default|GetIdleSounds))
    (CallFunction|RestartIdleSoundTimer 4.0)))

(fn ConstructionScript)

(fn Attack
  (Variables|Default|SetAttacking true)
  (Utilities|Time|SetTimerbyEvent (EventDispatchers|CreateEvent :!event Custom|OnAttackCooldownFinished) (Variables|Default|GetAttackCooldown))
  (if (Utilities|IsValid (Variables|Default|GetAttackSound))
    (Audio|SpawnSoundAttached (Variables|Default|GetAttackSound) (Variables|Character|GetMesh) "None" "0, 0, 0" "0, 0, 0" "KeepRelativeOffset" false 1.0 1.0 0.0 "/Game/Characters/Zombie/Audio/SA_ZombieGroan.SA_ZombieGroan" 0)))

(fn HandleSightSense
  (params (Actor :type Actor%20Object%20Reference) (Stimulus :type AI%20Stimulus%20Structure))
  (bind _returnvalue (Class|AIPerceptionSystem|GetSenseClassforStimulus Stimulus))
  (if (== _returnvalue "/Script/AIModule.AISense_Sight")
    (return (.bsuccessfullysensed Stimulus))
    (else
      (return false))))

(fn HandleDeath
  (params (Character :type BP%20Bombie%20Jackie%20Character%20Object%20Reference))
  (if (and (Variables|/Game/Characters/Jackie/BP_BombieJackieCharacter.BP_BombieJackieCharacter_C|GetIsDashing Character) (Variables|/Game/Characters/Jackie/BP_BombieJackieCharacter.BP_BombieJackieCharacter_C|GetbIsInSuperState Character))
    (Niagara|SpawnSystematLocation "/Game/Characters/NS_SuperKillEnemy.NS_SuperKillEnemy" (Transformation|GetActorLocation))
    (Utilities|IsValid (Variables|Default|GetDeathSound)
      (:Is%20Valid
        (Audio|PlaySound2D (Variables|Default|GetDeathSound) 1.0 1.0 0.0 0 0)
        (Actor|DestroyActor))
      (:Is%20Not%20Valid
        (Actor|DestroyActor)))
    (return true)
    (else
      (return false))))