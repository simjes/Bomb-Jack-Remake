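; BP_CoinSplosion is a one-shot effect actor that bursts a fountain of 50 coins at its location.
; On BeginPlay it plays the coin fountain sound, then spawns BP_Coin actors slightly above itself in a loop.
; Each coin's static mesh receives a velocity-change impulse in a random direction within an upward cone.
; The spawner calls DestroyActor on itself from inside the loop body.
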(event EventBeginPlay
  (Audio|SpawnSoundatLocation "/Game/Audio/SFX/SW_CoinFountain.SW_CoinFountain" (Transformation|GetActorLocation) "0, 0, 0" 1.0 1.0 0.0 0 0)
  (for _index (range 1 50)
    (bind _returnvalue (Game|SpawnActorfromClass "/Game/Object/Coin/BP_Coin.BP_Coin_C" (Math|Transform|MakeTransform (+ (Transformation|GetActorLocation) "0.000000,0.000000,40.000000")) "AdjustIfPossibleButAlwaysSpawn" "MultiplyWithRoot" 0 0))
    (Physics|AddImpulse (Actor|GetComponentbyClass _returnvalue "/Script/Engine.StaticMeshComponent") (* (Math|Random|RandomUnitVectorinConeinDegrees "0.000000,0.000000,1.000000" 45.0) 7.5e+02) "None" true)
    (Actor|DestroyActor)))

(fn ConstructionScript)