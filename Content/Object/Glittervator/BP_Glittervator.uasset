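; BP_Glittervator is a lift volume that propels BP_BombieJackieCharacter vertically while the character is inside it.
; Capsule overlap events store the character on entry and clear the reference on exit.
; While that reference is valid, Tick calls LaunchCharacter every frame with a Z-overriding velocity and calls EndHover with a cooldown reset.
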(event OnComponentBeginOverlap(Capsule)
  (params (OverlappedComponent :type Primitive%20Component%20Object%20Reference) (OtherActor :type Actor%20Object%20Reference) (OtherComp :type Primitive%20Component%20Object%20Reference) (OtherBodyIndex :type Integer) (bFromSweep :type Boolean) (SweepResult :type Hit%20Result%20Structure%20%28by%20ref%29))
  (bind _asbp_bombie_jackie_character (Utilities|Casting|CastToBP_BombieJackieCharacter OtherActor))
  (Variables|Default|SetCharacter _asbp_bombie_jackie_character))

(event OnComponentEndOverlap(Capsule)
  (params (OverlappedComponent :type Primitive%20Component%20Object%20Reference) (OtherActor :type Actor%20Object%20Reference) (OtherComp :type Primitive%20Component%20Object%20Reference) (OtherBodyIndex :type Integer))
  (Utilities|Casting|CastToBP_BombieJackieCharacter OtherActor)
  (Variables|Default|SetCharacter 0))

(event EventBeginPlay)

(event Collision|EventActorBeginOverlap
  (params (OtherActor :type Actor%20Object%20Reference)))

(event EventTick
  (params (DeltaSeconds :type Float%20%28single-precision%29))
  (bind _character (Variables|Default|GetCharacter))
  (Utilities|IsValid _character
    (:Is%20Valid
      (Character|LaunchCharacter _character (Math|Vector|MakeVector 0.0 0.0 (Variables|Default|GetLaunchVelocityZ)) false true)
      (Default|EndHover _character false true))))

(fn ConstructionScript)