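; Bomb pickup that the BombieJackie character defuses on overlap and that damages the pyramid when its lit fuse runs out.
; Overlap plays a sound and broadcasts the defusal, leaving removal outside this graph.
; LightFuse, run at BeginPlay if preset lit, swaps the mesh, enables custom depth and scales the bomb via timeline during the countdown.
; Explosion lowers pyramid HP through GameState, spawns effects, broadcasts and destroys the actor.
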(event OnComponentBeginOverlap(PickupCollision)
  (params (OverlappedComponent :type Primitive%20Component%20Object%20Reference) (OtherActor :type Actor%20Object%20Reference) (OtherComp :type Primitive%20Component%20Object%20Reference) (OtherBodyIndex :type Integer) (bFromSweep :type Boolean) (SweepResult :type Hit%20Result%20Structure%20%28by%20ref%29))
  (Utilities|Casting|CastToBP_BombieJackieCharacter OtherActor)
  (Audio|PlaySound2D "/Game/Object/Bomb/Audio/SW_BombDefuse.SW_BombDefuse" 1.0 1.0 0.0 0 0)
  (Default|CallBombDefused self))

(event Custom|LightFuse
  (Rendering|SetRenderCustomDepth (Variables|Default|GetStaticMesh) true)
  (Variables|Default|SetIsLit true)
  (Audio|SpawnSoundAttached "/Game/Object/Bomb/Audio/SW_BombFuse.SW_BombFuse" (Variables|Default|GetStaticMesh) "None" "0, 0, 0" "0, 0, 0" "KeepRelativeOffset" true 1.0 1.0 0.0 "/Game/Object/Bomb/Audio/SA_Bomb.SA_Bomb" 0)
  (Components|StaticMesh|SetStaticMesh (Variables|Default|GetStaticMesh) "/Game/Object/Bomb/Meshes/SM_LitBomb.SM_LitBomb")
  (Utilities|FlowControl|Sequence
    (:then_0
      (Utilities|FlowControl|Delay (Variables|Default|GetExplodeCountdown))
      (bind _asbp_bombie_jackie_game_state (Utilities|Casting|CastToBP_BombieJackieGameState (Game|GetGameState)))
      (Class|BombJackieGameState|DecreasePyramidHp _asbp_bombie_jackie_game_state (Variables|Default|GetDamage))
      (Audio|SpawnSoundAttached "/Game/Object/Bomb/Audio/SW_BombExplode.SW_BombExplode" (Variables|Default|GetStaticMesh) "None" "0, 0, 0" "0, 0, 0" "KeepRelativeOffset" false 1.0 1.0 0.0 "/Game/Object/Bomb/Audio/SA_Bomb.SA_Bomb" 0)
      (Niagara|SpawnSystematLocation "/Game/Object/Bomb/NS_BombExplosion.NS_BombExplosion" (Transformation|GetActorLocation))
      (Default|CallBombExploded self)
      (Utilities|FlowControl|Delay 0.1)
      (Actor|DestroyActor))
    (:then_1
      (bind _alpha (Timeline|Timeline Play)
        (:Update
          (Transformation|SetActorScale3D (Math|Vector|MakeVector (Math|Float|Lerp 0.8 1.2 _alpha) (Math|Float|Lerp 0.8 1.2 _alpha) (Math|Float|Lerp 0.8 1.2 _alpha))))))))

(event EventBeginPlay
  ;[0.15 0.15 0.15 0.5] Lights up bomb if set in details panel
  (if (Variables|Default|GetIsLit)
    (CallFunction|LightFuse)))

(fn ConstructionScript)