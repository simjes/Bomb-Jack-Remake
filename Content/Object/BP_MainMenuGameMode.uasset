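; Game mode for the main menu that shows the menu UI and applies saved settings on startup.
; On BeginPlay it sets the master sound mix, adds WBP_MainMenu to the viewport and loads GameUserSettings.
; If a settings save exists, it applies the saved music and SFX volumes as sound class overrides, then plays the menu theme.
; Without a valid save, the theme does not play.
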(event EventBeginPlay
  (bind _settingsslot (Variables|Default|GetSettingsSlot))
  (Class|GameplayStatics|SetBaseSoundMix "/Game/Audio/SCM_MasterMix.SCM_MasterMix")
  (bind _returnvalue (UserInterface|CreateWidget "/Game/UI/WBP_MainMenu.WBP_MainMenu_C" (Game|GetPlayerController 0)))
  (UserInterface|Viewport|AddtoViewport _returnvalue 0)
  (bind _returnvalue_2 (Settings|GetGameUserSettings))
  (Class|GameUserSettings|LoadSettings _returnvalue_2 false)
  (bind _returnvalue_3 (SaveGame|DoesSaveGameExist _settingsslot))
  (if _returnvalue_3
    (bind _returnvalue_4 (SaveGame|LoadGamefromSlot _settingsslot))
    (bind _asbp_settings_save (Utilities|Casting|CastToBP_SettingsSave _returnvalue_4))
    (Audio|SetSoundMixClassOverride "/Game/Audio/SCM_MasterMix.SCM_MasterMix" "/Game/Audio/Music/SC_MasterMusic.SC_MasterMusic" (Variables|/Game/SaveGame/BP_SettingsSave.BP_SettingsSave_C|GetMusicSound _asbp_settings_save) 1.0 1.0 true)
    (Audio|SetSoundMixClassOverride "/Game/Audio/SCM_MasterMix.SCM_MasterMix" "/Game/Audio/SFX/SC_MasterSFX.SC_MasterSFX" (Variables|/Game/SaveGame/BP_SettingsSave.BP_SettingsSave_C|GetSFXSound _asbp_settings_save) 1.0 1.0 true)
    (Audio|PlaySound2D "/Game/Audio/Music/SW_MenuTheme.SW_MenuTheme" 1.0 1.0 0.0 0 0)))

(event EventTick
  (params (DeltaSeconds :type Float%20%28single-precision%29)))

(fn ConstructionScript)