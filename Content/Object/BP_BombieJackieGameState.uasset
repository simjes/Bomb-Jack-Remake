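; Game state for a bomb-defusing game that tracks every BP_Bomb in the level and triggers victory once each one is defused or exploded.
; On BeginPlay it binds to each bomb's events and starts the fuse cycle unless one is pre-lit.
; Explosions and lit-bomb defusals schedule another fuse after a random delay, preferring bombs near the player.
; Removed bombs are destroyed and the remaining count is broadcast.
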(event Custom|HandleBombExploded
  (params (Instigator :type BP%20Bomb%20Object%20Reference))
  (Variables|Default|SetExplodedBombs (+ (Variables|Default|GetExplodedBombs) 1))
  (CallFunction|CleanupRemovedBomb Instigator)
  (CallFunction|OnLightUpBombDelayed)
  (bind _winningconditionsmet (CallFunction|CheckWinCondition))
  (if _winningconditionsmet
    (Class|BombJackieGameState|HandleVictory)))

(event Custom|HandleBombDefused
  (params (Instigator :type BP%20Bomb%20Object%20Reference))
  (Variables|Default|SetDefusedBombs (+ (Variables|Default|GetDefusedBombs) 1))
  (Utilities|FlowControl|Sequence
    (:then_0
      (bind _winningconditionsmet (CallFunction|CheckWinCondition))
      (if _winningconditionsmet
        (Class|BombJackieGameState|HandleVictory)))
    (:then_1
      (if (Variables|/Game/Object/Bomb/BP_Bomb.BP_Bomb_C|GetIsLit Instigator)
        (CallFunction|CleanupRemovedBomb Instigator)
        (CallFunction|OnLightUpBombDelayed)
        (else
          (CallFunction|CleanupRemovedBomb Instigator))))))

(event Custom|OnLightUpBombDelayed
  (Utilities|Time|SetTimerbyEvent (delegate Custom|CallLightUpRandomBomb) (Math|Random|RandomFloatinRange (Variables|Default|GetMinBombLightDelay) (Variables|Default|GetMaxBombLightDelay))))

(event Custom|CallLightUpRandomBomb
  (CallFunction|LightRandomBomb))

(event EventBeginPlay
  (bind _outactors (Actor|GetAllActorsOfClass "/Game/Object/Bomb/BP_Bomb.BP_Bomb_C"))
  (bind _output_get (Variables|Default|SetRemainingBombs _outactors))
  (bind _output_get_2 (Variables|Default|SetTotalBombs (Utilities|Array|Length _output_get)))
  (Utilities|FlowControl|Sequence
    (:then_0
      (Class|BombJackieGameState|BroadcastBombsChanged _output_get_2))
    (:then_1
      ;[0.15 0.15 0.15 0.5] Light up a bomb if none is lit by the developer
      (bind _array_element (Utilities|Array|ForEachLoopwithBreak _outactors :!label _label)
        (:LoopBody
          (if (Variables|/Game/Object/Bomb/BP_Bomb.BP_Bomb_C|GetIsLit _array_element)
            (Variables|Default|SetShouldLightBomb false)
            (goto _label Break)))
        (:Completed
          (if (Variables|Default|GetShouldLightBomb)
            (CallFunction|OnLightUpBombDelayed)))))
    (:then_2
      ;[0.15 0.15 0.15 0.5] Bind events for exploded or defused bombs
      (for _array_element_2 _outactors
        (EventDispatchers|BindEventtoBombDefused _array_element_2 (delegate Custom|HandleBombDefused))
        (EventDispatchers|BindEventtoBombExploded _array_element_2 (delegate Custom|HandleBombExploded))))))

(fn ConstructionScript)

(fn LightRandomBomb
  (if (!= (Utilities|Array|Length (Variables|Default|GetRemainingBombs)) 0)
    (for _array_element (Variables|Default|GetRemainingBombs)
      (if (<= (Math|Vector|Distance(Vector) (Transformation|GetActorLocation _array_element) (Transformation|GetActorLocation (Game|GetPlayerCharacter 0))) (Variables|Default|GetPlayerBombRadius))
        (Utilities|Array|Add (Variables|Default|GetBombsInCharacterRange) _array_element)))
    (if (> (Utilities|Array|Length (Variables|Default|GetBombsInCharacterRange)) 0)
      (Default|LightFuse (.OutItem (Utilities|Array|Random (Variables|Default|GetBombsInCharacterRange))))
      (Utilities|Array|Clear (Variables|Default|GetBombsInCharacterRange))
      (else
        (Default|LightFuse (.OutItem (Utilities|Array|Random (Variables|Default|GetRemainingBombs))))))))

(fn CheckWinCondition
  (return (== (Variables|Default|GetDefusedBombs) (- (Variables|Default|GetTotalBombs) (Variables|Default|GetExplodedBombs)))))

(fn CleanupRemovedBomb
  (params (BombToClean :type BP%20Bomb%20Object%20Reference))
  (Utilities|Array|RemoveItem (Variables|Default|GetRemainingBombs) BombToClean)
  (Actor|DestroyActor BombToClean)
  (Class|BombJackieGameState|BroadcastBombsChanged (Utilities|Array|Length (Variables|Default|GetRemainingBombs))))